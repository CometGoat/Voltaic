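; Timed map hazard that periodically electrifies water, killing overlapping players up to a per-activation charge limit.
; BeginPlay gathers doors, lights and billboards, then polls game state before running a randomized, Tick-driven countdown.
; Warnings start alarm, lights and billboards, doors close, then timelines drive the water material while collision is live, before resetting.
; A mode-specific controller is spawned without a pawn as the hazard's named killer identity.
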(event OnComponentBeginOverlap(ElectricityPlane)
  (params (OverlappedComponent :type Primitive%20Component%20Object%20Reference) (OtherActor :type Actor%20Object%20Reference) (OtherComp :type Primitive%20Component%20Object%20Reference) (OtherBodyIndex :type Integer) (bFromSweep :type Boolean) (SweepResult :type Hit%20Result%20Structure%20%28by%20ref%29))
  (bind _hazardcontroller (Variables|Default|GetHazardController))
  (if (not (or (<= (Variables|Default|GetCharge) 0) (== OtherActor (Variables|Default|GetHazardController))))
    ;[1 1 1] Colliding with mesh when hazard is active kills player
    (Variables|Default|SetCharge (- (Variables|Default|GetCharge) 1))
    (bind _asetcplayer_character (Utilities|Casting|CastToETCPlayerCharacter OtherActor)
      (:then
        (Default|Death _asetcplayer_character))
      (:CastFailed
        (bind _asdeathmatch_character_split (Utilities|Casting|CastToDeathmatchCharacter_Split OtherActor)
          (:then
            ;[1 1 1] Activating the hazard
            (Default|Death _asdeathmatch_character_split _hazardcontroller))
          (:CastFailed
            (bind _asetcplayer_character_split (Utilities|Casting|CastToETCPlayerCharacter_Split OtherActor))
            (Default|Death _asetcplayer_character_split _hazardcontroller)))))))

(event Custom|BeginCountdown
  ;[1 1 1] Timer counting down to hazard event
  (Utilities|FlowControl|Gate true) ; enters at Open
)

(event Custom|CreateHazardEntity
  (switch int (Variables|/Game/Gameplay/SaveData/ETC_GameInstance.ETC_GameInstance_C|GetModeID (.AsETC%20Game%20Instance (Utilities|Casting|CastToETC_GameInstance (Game|GetGameInstance))))
    (:0
      (bind _returnvalue (Game|SpawnActorfromClass "/Game/Player/Controllers/ETCPlayerController_Split.ETCPlayerController_Split_C" (Math|Transform|MakeTransform "0,0.000000, 0") "Undefined" 0 true 0 :!label _label))
      (Actor|Tick|SetActorTickEnabled _returnvalue true)
      (bind _output_get (Variables|Default|SetHazardController _returnvalue))
      (Utilities|IsValid _output_get
        (:Is%20Valid
          (Utilities|IsValid (Pawn|GetControlledPawn _output_get)
            (:Is%20Valid
              (Actor|DestroyActor (Pawn|GetControlledPawn _output_get)))
            (:Is%20Not%20Valid
              _))
          (Utilities|FlowControl|Delay 1.0)
          (Variables|/Game/Player/PlayerStates/ETC_PlayerState_Split.ETC_PlayerState_Split_C|SetPlayerName%20%28Temporary%29 (.AsETC%20Player%20State%20Split (Utilities|Casting|CastToETC_PlayerState_Split (Variables|/Script/Engine.Controller|GetPlayerState _output_get))) (Variables|Default|GetHazardName)))
        (:Is%20Not%20Valid
          (Development|PrintString "Not valid!")
          (Utilities|FlowControl|Delay 1.0)
          (goto _label))))
    (:1
      (bind _returnvalue_2 (Game|SpawnActorfromClass "/Game/Player/Controllers/DeathmatchController_Split.DeathmatchController_Split_C" (Math|Transform|MakeTransform "0,0.000000, 0") "Undefined" 0 true 0 :!label _label_2))
      (Actor|Tick|SetActorTickEnabled _returnvalue_2 true)
      (bind _output_get_2 (Variables|Default|SetHazardController _returnvalue_2))
      (Utilities|IsValid _output_get_2
        (:Is%20Valid
          (Utilities|IsValid (Pawn|GetControlledPawn _output_get_2)
            (:Is%20Valid
              (Actor|DestroyActor (Pawn|GetControlledPawn _output_get_2)))
            (:Is%20Not%20Valid
              _))
          (Utilities|FlowControl|Delay 1.0)
          (Variables|/Game/Player/PlayerStates/DeathmatchPlayerState_Split.DeathmatchPlayerState_Split_C|SetPlayerName%20%28Temporary%29 (.AsDeathmatch%20Player%20State%20Split (Utilities|Casting|CastToDeathmatchPlayerState_Split (Variables|/Script/Engine.Controller|GetPlayerState _output_get_2))) (Variables|Default|GetHazardName)))
        (:Is%20Not%20Valid
          (Development|PrintString "Not valid!")
          (Utilities|FlowControl|Delay 1.0)
          (goto _label_2))))
    (:2
      (bind _returnvalue_3 (Game|SpawnActorfromClass "/Game/Player/Controllers/ETCPlayerController.ETCPlayerController_C" (Math|Transform|MakeTransform "0,0.000000, 0") "Undefined" 0 true 0 :!label _label_3))
      (Actor|Tick|SetActorTickEnabled _returnvalue_3 true)
      (bind _output_get_3 (Variables|Default|SetHazardController _returnvalue_3))
      (Utilities|IsValid _output_get_3
        (:Is%20Valid
          (Utilities|IsValid (Pawn|GetControlledPawn _output_get_3) :!label _label_4
            (:Is%20Valid
              (Actor|DestroyActor (Pawn|GetControlledPawn _output_get_3))
              (Utilities|FlowControl|Delay 1.0)
              (Variables|/Game/Player/PlayerStates/ETC_PlayerState.ETC_PlayerState_C|SetPlayerName%20%28Temporary%29 (.AsETC%20Player%20State (Utilities|Casting|CastToETC_PlayerState (Variables|/Script/Engine.Controller|GetPlayerState _output_get_3))) (Variables|Default|GetHazardName)))
            (:Is%20Not%20Valid
              (Utilities|FlowControl|Delay 0.1)
              (goto _label_4))))
        (:Is%20Not%20Valid
          (Development|PrintString "Not valid!")
          (Utilities|FlowControl|Delay 1.0)
          (goto _label_3))))))

(event Custom|ActivateHazard
  (bind _electrifiedwater (Variables|Default|GetElectrifiedWater))
  ;[1 1 1] Activating the hazard
  (Audio|PlaySound2D "/Game/Sounds/Cues/S_OBJ_ElecChargeUp_Cue.S_OBJ_ElecChargeUp_Cue")
  ;[1 1 1] Delay for sound
  (Utilities|FlowControl|Delay 2.0)
  (Audio|PlaySound2D "/Game/Sounds/Cues/S_OBJ_ElecDischarge_Cue.S_OBJ_ElecDischarge_Cue")
  (bind _returnvalue (Audio|SpawnSound2D "/Game/Sounds/Cues/S_OBJ_ElecFloorLoop_Cue.S_OBJ_ElecFloorLoop_Cue"))
  ;[1 1 1] Activates Collision
  (Collision|SetCollisionEnabled (Variables|Default|GetElectricityPlane) "QueryAndPhysics")
  (Rendering|Material|SetScalarParameterValue (Variables|Default|GetElectrifiedWater) "WaterColour" 1.0 :!class /Script/Engine.MaterialInstanceDynamic)
  (bind (_direction _electricity _electricityopactity) (Timeline|IncreaseBrightness PlayFromStart)
    (:Update
      (Rendering|Material|SetScalarParameterValue _electrifiedwater "ElectricityBrightness" _electricity :!class /Script/Engine.MaterialInstanceDynamic)
      (Rendering|Material|SetScalarParameterValue _electrifiedwater "ElectricityOpacity" _electricityopactity :!class /Script/Engine.MaterialInstanceDynamic))
    (:Finished
      ;[1 1 1] Duration
      (Utilities|FlowControl|Delay 4.0)
      (Audio|Components|Audio|Stop _returnvalue)
      (Components|DestroyComponent _returnvalue)
      (Audio|PlaySound2D "/Game/Sounds/Cues/S_OBJ_ElecOff_Cue.S_OBJ_ElecOff_Cue")
      ;[1 1 1] Disables collision and resets countdown
      (Collision|SetCollisionEnabled (Variables|Default|GetElectricityPlane) "NoCollision")
      (for _array_element (Variables|Default|GetDoors)
        (Default|OpenDoors _array_element))
      (for _array_element_2 (Variables|Default|GetSpinningLights)
        (Default|StopRotation _array_element_2))
      (CallFunction|SetTimerNew)
      (bind _newtrack_1 (Timeline|PowerDown PlayFromStart)
        (:Update
          (Rendering|Material|SetScalarParameterValue (Variables|Default|GetElectrifiedWater) "ElectricityOpacity" _newtrack_1 :!class /Script/Engine.MaterialInstanceDynamic))))))

(event Custom|HazardCountdownSFX
  (params (Countdown :type Integer))
  (bind _returnvalue (- Countdown 1))
  (Audio|PlaySound2D "/Game/Sounds/Cues/S_AMB_HazardAlarm_Cue.S_AMB_HazardAlarm_Cue")
  (if (not (< _returnvalue 0))
    (Utilities|FlowControl|Delay 1.0)
    (CallFunction|HazardCountdownSFX _returnvalue)))

(event EventBeginPlay
  (bind _returnvalue (Game|GetGameState))
  ;[1 1 1] Getting all doors, spinning lights and billboards
  (CallFunction|GrabbingRelevantActors)
  (CallFunction|CreateHazardEntity)
  ;[1 1 1] Sets intial Timer, delay can be removed when the next section is created with an event dispatcher
  (Utilities|FlowControl|Delay 0.2)
  (CallFunction|SetTimerNew)
  (bind _returnvalue_2 (Rendering|Material|CreateDynamicMaterialInstance (Variables|Default|GetElectricityPlane) 0 "/Game/Environment/Materials/WaterShader/M_WaterShader_Inst.M_WaterShader_Inst" :!class /Script/Engine.PrimitiveComponent))
  (Variables|Default|SetElectrifiedWater _returnvalue_2)
  ;[1 0 0] This could be done much more efficiently with an event dispatcher, will redo.
  (bind _asetc_game_state (Utilities|Casting|CastToETC_GameState _returnvalue :!label _label)
    (:then
      (if (Utilities|Enum|Equal(Enum) (Variables|/Game/Gameplay/GameStates/ETC_GameState.ETC_GameState_C|GetGameplayState _asetc_game_state) "NewEnumerator2")
        _
        (else
          (Utilities|FlowControl|Delay 0.2 :!label _label_2)
          (goto _label))))
    (:CastFailed
      (bind _asdeathmatch_game_state_split (Utilities|Casting|CastToDeathmatchGameState_Split _returnvalue)
        (:then
          (if (Utilities|Enum|Equal(Enum) (Variables|/Game/Gameplay/GameStates/DeathmatchGameState_Split.DeathmatchGameState_Split_C|GetGameplayState_Split _asdeathmatch_game_state_split) "NewEnumerator2")
            _
            (else
              (goto _label_2))))
        (:CastFailed
          (bind _asetc_game_state_split (Utilities|Casting|CastToETC_GameState_Split _returnvalue))
          (if (Utilities|Enum|Equal(Enum) (Variables|/Game/Gameplay/GameStates/ETC_GameState_Split.ETC_GameState_Split_C|GetGameplayState_Split _asetc_game_state_split) "NewEnumerator2")
            _
            (else
              (goto _label_2)))))))
  (CallFunction|BeginCountdown))

(event EventTick
  (params (DeltaSeconds :type Float%20%28single-precision%29))
  ;[1 1 1] Timer counting down to hazard event
  (if (not (Variables|Default|GetEventActive))
    (Utilities|FlowControl|Gate true
      (:Exit
        (bind _output_get (Variables|Default|SetTimeRemaining (Math|Float|Max(Float) (- (Variables|Default|GetTimeRemaining) DeltaSeconds) 0.0)))
        (if (<= _output_get 0.0)
          ;[1 1 1] Activating events associated with hazards
          (Variables|Default|SetEventActive true)
          (Variables|Default|SetCharge 4)
          (CallFunction|ActivateHazard)
          (Utilities|FlowControl|Sequence
            (:then_0
              (goto _label Reset))
            (:then_1
              (goto _label_2 Reset)))
          (elif (<= (Variables|Default|GetTimeRemaining) 1.0)
            (Utilities|FlowControl|DoOnce false :!label _label
              (:Completed
                (for _array_element (Variables|Default|GetDoors)
                  (Default|CloseDoors _array_element))))
            (elif (<= (Variables|Default|GetTimeRemaining) 9.0)
              (Utilities|FlowControl|DoOnce false :!label _label_2
                (:Completed
                  (for _array_element_2 (Variables|Default|GetSpinningLights)
                    (Default|StartRotation _array_element_2))
                  (for _array_element_3 (Variables|Default|GetBillboards)
                    (Default|ChangeBillboardImage _array_element_3))
                  (Rendering|Material|SetScalarParameterValue (Variables|Default|GetElectrifiedWater) "WaterColour" 0.0 :!class /Script/Engine.MaterialInstanceDynamic)
                  (CallFunction|HazardCountdownSFX 10))))))))))

(fn ConstructionScript)

(fn SetTimerNew
  (Variables|Default|SetTimeRemaining (Math|Conversions|ToFloat(Integer) (Math|Float|Truncate (Math|Random|RandomFloatinRange (Variables|Default|GetMinTimeBeforeEvent) (Variables|Default|GetMaxTimeBeforeEvent)))))
  (Variables|Default|SetEventActive false))

(fn GrabbingRelevantActors
  (bind _outactors (Actor|GetAllActorsOfClass "/Game/Environment/BlueprintsEnvironment/BP_ClosingDoors.BP_ClosingDoors_C"))
  (Variables|Default|SetDoors _outactors)
  (bind _outactors_2 (Actor|GetAllActorsOfClass "/Game/Environment/BlueprintsEnvironment/BP_SpinningLights.BP_SpinningLights_C"))
  (Variables|Default|SetSpinningLights _outactors_2)
  (bind _outactors_3 (Actor|GetAllActorsOfClass "/Game/Environment/BlueprintsEnvironment/BP_Billboards.BP_Billboards_C"))
  (Variables|Default|SetBillboards _outactors_3))