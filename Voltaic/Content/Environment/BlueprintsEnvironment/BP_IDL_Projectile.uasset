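; BP_IDL_Projectile is a bouncing projectile actor that destroys itself after a limited number of bounces.
; On BeginPlay it sets the TeamColor parameter of its particle ribbon to a hardcoded white.
; Each bounce event from the projectile movement component calls CountBounce, which decrements Bounces and destroys the actor once none remain.
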(event OnProjectileBounce(ProjectileMovement)
  (params (ImpactResult :type Hit%20Result%20Structure%20%28by%20ref%29) (ImpactVelocity :type Vector%20%28by%20ref%29 :default "0, 0, 0"))
  ;[1 1 1] On Projectile Bounce
  (|CountBounce))

(event EventBeginPlay
  ;[1 1 1] Set Team Colour
  (Effects|Components|ParticleSystem|SetColorParameter (Variables|Default|GetParticle_Ribbon) "TeamColor" "(R=1.000000,G=1.000000,B=1.000000,A=1.000000)"))

(event Collision|EventActorBeginOverlap
  (params (OtherActor :type Actor%20Object%20Reference)))

(event EventTick
  (params (DeltaSeconds :type Float%20%28single-precision%29)))

(fn ConstructionScript)