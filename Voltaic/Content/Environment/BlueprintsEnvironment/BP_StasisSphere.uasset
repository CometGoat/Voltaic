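; BP_StasisSphere is the expanding stasis pulse of a BP_StasisTrap, stunning player characters it touches other than the trap's owner.
; On BeginPlay a timeline scales the actor up sixtyfold around its location, then destroys it when finished.
; Mesh overlaps resolve the player through the overlapping actor's Instigator before calling Stun.
; The construction script gives the mesh a dynamic material tinted by PulseColour.
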(event OnComponentBeginOverlap(StaticMesh)
  (params (OverlappedComponent :type Primitive%20Component%20Object%20Reference) (OtherActor :type Actor%20Object%20Reference) (OtherComp :type Primitive%20Component%20Object%20Reference) (OtherBodyIndex :type Integer) (bFromSweep :type Boolean) (SweepResult :type Hit%20Result%20Structure%20%28by%20ref%29))
  (bind _asetcplayer_character (Utilities|Casting|CastToETCPlayerCharacter (Variables|/Script/Engine.Actor|GetInstigator OtherActor)))
  (if (not (== (Components|GetOwner (.AsBP%20Stasis%20Trap (Utilities|Casting|CastToBP_StasisTrap (Components|GetOwner)))) _asetcplayer_character))
    (Default|Stun _asetcplayer_character)))

(event EventBeginPlay
  (bind _newtrack_0 (Timeline|Timeline_0 PlayFromStart)
    (:Update
      (Transformation|SetActorTransform (Math|Transform|Lerp(Transform) (Math|Transform|MakeTransform (Transformation|GetActorLocation)) (Math|Transform|MakeTransform (Transformation|GetActorLocation) "0, 0, 0" "60.000000,60.000000,60.000000") _newtrack_0)))
    (:Finished
      (Actor|DestroyActor))))

(fn ConstructionScript
  (bind _returnvalue (Rendering|Material|CreateDynamicMaterialInstance (Variables|Default|GetStaticMesh) 0 "/Game/Environment/Materials/M_StasisSphere_Inst.M_StasisSphere_Inst" :!class /Script/Engine.PrimitiveComponent))
  (Rendering|Material|SetVectorParameterValue _returnvalue "PulseColour" (Variables|Default|GetPulseColour) :!class /Script/Engine.MaterialInstanceDynamic))