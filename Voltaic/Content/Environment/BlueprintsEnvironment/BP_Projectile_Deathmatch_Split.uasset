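; Team-coloured deathmatch projectile that registers with the game state, ricochets a limited number of times and damages enemy characters it overlaps.
; Dodging characters reverse its velocity, with an enemy's dodge also switching its team and colour.
; Bounces cache fast velocities, which are reversed and restored if movement stops.
; It counts its kills to trigger double and triple kill announcements, and fades its sound out on destruction.
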(event OnComponentBeginOverlap(ProjectileCollision)
  (params (OverlappedComponent :type Primitive%20Component%20Object%20Reference) (OtherActor :type Actor%20Object%20Reference) (OtherComp :type Primitive%20Component%20Object%20Reference) (OtherBodyIndex :type Integer) (bFromSweep :type Boolean) (SweepResult :type Hit%20Result%20Structure%20%28by%20ref%29))
  (bind _returnvalue (Game|GetGameMode))
  (bind _asdeathmatch_game_mode_split (Utilities|Casting|CastToDeathmatch_GameMode_Split _returnvalue))
  (bind _asdeathmatch_character_split (Utilities|Casting|CastToDeathmatchCharacter_Split (Variables|/Script/Engine.Actor|GetInstigator OtherActor)))
  ;[1 1 1] Detecting Hits
  (if (== (Variables|Default|GetTeamNum) (Math|Conversions|ToByte(Integer) (Variables|/Game/Player/Pawns/DeathmatchCharacter_Split.DeathmatchCharacter_Split_C|GetTeamCount _asdeathmatch_character_split)))
    (CallFunction|ReflectOwnTeam _asdeathmatch_character_split)
    (elif (Variables|/Game/Player/Pawns/DeathmatchCharacter_Split.DeathmatchCharacter_Split_C|GetDodging? _asdeathmatch_character_split)
      (CallFunction|ReflectOtherTeam _asdeathmatch_character_split)
      (else
        (Utilities|IsValid (Variables|/Game/Player/Pawns/DeathmatchCharacter_Split.DeathmatchCharacter_Split_C|GetPlayerIndicatorWidget _asdeathmatch_character_split)
          (:Is%20Valid
            (Default|Remove (Variables|/Game/Player/Pawns/DeathmatchCharacter_Split.DeathmatchCharacter_Split_C|GetPlayerIndicatorWidget _asdeathmatch_character_split)))
          (:Is%20Not%20Valid
            _))
        (Utilities|IsValid OtherActor
          (:Is%20Valid
            (Game|Damage|ApplyDamage OtherActor 1.0 (Game|GetInstigatorController) self)
            (bind _returnvalue_2 (Effects|SpawnEmitteratLocation "/Game/Effects/Particles/P_DeathParticle_2.P_DeathParticle_2" (Transformation|GetActorLocation)))
            (Effects|Components|ParticleSystem|SetColorParameter _returnvalue_2 "SparkColour" (Variables|Default|GetParticleColour))
            (bind _output_get (Variables|Default|SetKillCount (+ (Variables|Default|GetKillCount) 1)))
            (if (== _output_get 2)
              (Default|AnnouncerDoubleKill _asdeathmatch_game_mode_split)
              (elif (== _output_get 3)
                (Default|AnnouncerTripleKill _asdeathmatch_game_mode_split)))))))))

(event OnProjectileBounce(ProjectileMovement)
  (params (ImpactResult :type Hit%20Result%20Structure%20%28by%20ref%29) (ImpactVelocity :type Vector%20%28by%20ref%29 :default "0, 0, 0"))
  (bind _returnvalue (Transformation|GetVelocity))
  (bind (_x _y _z) (Math|Vector|BreakVector _returnvalue))
  ;[1 1 1] Counting Bounces
  (if (Utilities|IsValid (.HitActor (Collision|BreakHitResult ImpactResult)))
    (Variables|Default|SetNumberOfBounces (- (Variables|Default|GetNumberOfBounces) 1))
    (Effects|SpawnEmitteratLocation "/Game/Effects/Particles/P_Ricochet.P_Ricochet" (Transformation|GetActorLocation) (Transformation|GetActorRotation))
    (if (<= (Variables|Default|GetNumberOfBounces) 0)
      (CallFunction|DestroyActor)
      (elif (or (> (Math|Float|Absolute(Float) _x) 2e+03) (> (Math|Float|Absolute(Float) _y) 2e+03))
        (Variables|Default|SetCurrentVelocity _returnvalue)))))

(event OnProjectileStop(ProjectileMovement)
  (params (ImpactResult :type Hit%20Result%20Structure%20%28by%20ref%29))
  (Utilities|FlowControl|Delay 0.0)
  (CallFunction|ResetVeolicty))

(event Custom|DestroyActor
  ;[1 1 1] Counting Bounces
  (Components|DestroyComponent (Variables|Default|GetProjectileMesh))
  (Audio|Components|Audio|FadeOut (Variables|Default|GetProjectileSound) 1.0 0.0 :!class /Script/Engine.AudioComponent)
  (Utilities|FlowControl|Delay 2.0)
  (Actor|DestroyActor))

(event Custom|Reflect_OwnTeam
  (params (Character :type Deathmatch%20Character%20Split%20Object%20Reference))
  (if (and (Variables|/Game/Player/Pawns/DeathmatchCharacter_Split.DeathmatchCharacter_Split_C|GetDodging? Character) (not (Variables|Default|GetReflected_OwnTeam)))
    (Variables|Default|SetReflected_OwnTeam true)
    (Variables|/Script/Engine.MovementComponent|SetVelocity (Variables|Default|GetProjectileMovement) (Math|Vector|RotateVector (Transformation|GetVelocity) "0.000000,180.000000,0.000000"))
    (Audio|PlaySoundatLocation "/Game/Sounds/Cues/Player_Reflect.Player_Reflect" (Transformation|GetActorLocation self))
    (Utilities|FlowControl|Delay 0.2)
    (Variables|Default|SetReflected_OwnTeam false)))

(event Custom|ResetVeolicty
  (bind _projectilemovement (Variables|Default|GetProjectileMovement))
  (Components|Movement|SetUpdatedComponent _projectilemovement (Variables|Default|GetProjectileCollision))
  (Variables|/Script/Engine.MovementComponent|SetVelocity _projectilemovement (Math|Vector|RotateVector (Variables|Default|GetCurrentVelocity) "0.000000,180.000000,0.000000")))

(event Custom|Reflect_OtherTeam
  (params (Character :type Deathmatch%20Character%20Split%20Object%20Reference))
  (bind _cachedteaminfo (Variables|/Game/Player/Pawns/DeathmatchCharacter_Split.DeathmatchCharacter_Split_C|GetCachedTeamInfo Character))
  (bind _teamcolour (Variables|/Game/Gameplay/BlueprintsGameplay/TeamInfo/BaseTeamInfo.BaseTeamInfo_C|GetTeamColour _cachedteaminfo))
  (Variables|Default|SetReflected_OwnTeam true)
  (Variables|/Script/Engine.MovementComponent|SetVelocity (Variables|Default|GetProjectileMovement) (Math|Vector|RotateVector (Transformation|GetVelocity) "0.000000,180.000000,0.000000"))
  (Variables|Default|SetTeamNum (Math|Conversions|ToByte(Integer) (Variables|/Game/Player/Pawns/DeathmatchCharacter_Split.DeathmatchCharacter_Split_C|GetTeamCount Character)))
  (Effects|Components|ParticleSystem|SetColorParameter (Variables|Default|GetParticleSystem) "TeamColor" _teamcolour)
  (Rendering|Components|Light|SetLightColor (Variables|Default|GetPointLight) _teamcolour true)
  (Audio|PlaySoundatLocation "/Game/Sounds/Cues/Player_Reflect.Player_Reflect" (Transformation|GetActorLocation self))
  (Utilities|FlowControl|Delay 0.2)
  (Variables|Default|SetReflected_OwnTeam false))

(event EventBeginPlay
  (bind _returnvalue (Game|GetGameState))
  (bind _returnvalue_2 (Components|GetOwner))
  (bind _particlecolour (Variables|Default|GetParticleColour))
  (bind _asdeathmatch_game_state_split (Utilities|Casting|CastToDeathmatchGameState_Split _returnvalue))
  (bind _instigator (Variables|/Script/Engine.Actor|GetInstigator _returnvalue_2))
  ;[1 1 1] Set Projectile Ribbon Color
  (Variables|Default|SetOwningPlayerController (Pawn|GetController _instigator))
  (Variables|Default|SetTeamNum (Math|Conversions|ToByte(Integer) (Variables|/Game/Player/Pawns/DeathmatchCharacter_Split.DeathmatchCharacter_Split_C|GetTeamCount (.AsDeathmatch%20Character%20Split (Utilities|Casting|CastToDeathmatchCharacter_Split _instigator)))))
  (Audio|Components|Audio|Play (Variables|Default|GetProjectileSound) 0.0)
  (Effects|Components|ParticleSystem|SetColorParameter (Variables|Default|GetParticleSystem) "TeamColor" _particlecolour)
  (Rendering|Components|Light|SetLightColor (Variables|Default|GetPointLight) _particlecolour true)
  ;[1 1 1] Add Self to ProjectileList
  (Variables|/Game/Gameplay/GameStates/DeathmatchGameState_Split.DeathmatchGameState_Split_C|SetProjectileToAdd _asdeathmatch_game_state_split self)
  (Default|AddtoProjectileList _asdeathmatch_game_state_split))

(event EventDestroyed
  (Audio|Components|Audio|FadeOut (Variables|Default|GetProjectileSound) 0.1 0.0 :!class /Script/Engine.AudioComponent))

(fn ConstructionScript
  ;[1 1 1] Always spawns on the server because of how we are spawning projectiles
)

(fn ReflectOffPlayer
  (params (HitCharacter :type Deathmatch%20Character%20Split%20Object%20Reference))
  (if (Variables|/Game/Player/Pawns/DeathmatchCharacter_Split.DeathmatchCharacter_Split_C|GetDodging? HitCharacter)
    (Game|Components|ProjectileMovement|SetVelocityinLocalSpace (Variables|Default|GetProjectileMovement) (Math|Vector|RotateVector (Transformation|GetVelocity) "0,180.000000, 0"))
    (Development|PrintString "Reflected!")))