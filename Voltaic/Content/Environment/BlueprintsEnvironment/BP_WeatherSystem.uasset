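; BP_WeatherSystem is a storm actor that, when Storm is set, activates rain and starts lightning and thunder on BeginPlay.
; Lightning waits, plays a timeline that drives light intensity, then re-randomizes both delays and calls itself and Thunder.
; Thunder timing varies around the new lightning interval.
; Its sound plays at a fixed height, with X and Y derived from the actor's location randomly scaled and rotated.
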(event Custom|Lightning
  (bind _delayeitherside (Variables|Default|GetDelayEitherSide))
  (Utilities|FlowControl|Delay (Variables|Default|GetTimeBetweenLightning))
  (bind _lightning (Timeline|Timeline_0 PlayFromStart)
    (:Update
      (Rendering|Components|Light|SetIntensity (Variables|Default|GetLightComponent) (* _lightning 2.0)))
    (:Finished
      (Variables|Default|SetTimeBetweenLightning (Math|Random|RandomFloatinRange 11.0 19.0))
      (Variables|Default|SetTimeBetweenThunder (Math|Random|RandomFloatinRange (- (Variables|Default|GetTimeBetweenLightning) _delayeitherside) (+ (Variables|Default|GetTimeBetweenLightning) _delayeitherside)))
      (CallFunction|Lightning)
      (CallFunction|Thunder))))

(event Custom|Thunder
  (bind _returnvalue (Math|Random|RandomRotator false))
  (bind _returnvalue_2 (Transformation|GetActorLocation))
  (bind _maximumdistance (Variables|Default|GetMaximumDistance))
  (bind _minimumdistance (Variables|Default|GetMinimumDistance))
  (bind _returnvalue_3 (Math|Random|RandomFloatinRange _minimumdistance _maximumdistance))
  (bind _returnvalue_4 (* _returnvalue_2 _returnvalue_3))
  (bind _returnvalue_5 (Math|Vector|RotateVector _returnvalue_4 _returnvalue))
  (Utilities|FlowControl|Delay (Variables|Default|GetTimeBetweenThunder))
  (Audio|PlaySoundatLocation "/Game/Sounds/Cues/S_Thunder_Cue.S_Thunder_Cue" (Math|Vector|MakeVector (.x _returnvalue_5) (.y _returnvalue_5) 4e+03)))

(event EventBeginPlay
  (if (Variables|Default|GetStorm?)
    (CallFunction|Lightning)
    (CallFunction|Thunder)
    (Components|Activation|Activate (Variables|Default|GetRain) false)))

(fn ConstructionScript)