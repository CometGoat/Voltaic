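; BP_SpinningLights is a spinning light fixture with two spotlights and a rotating cylinder, switched on and off through events.
; StartRotation shows the spotlights and opens a gate on Tick, and StopRotation hides them and closes it.
; While the gate is open, the cylinder turns a fixed step every frame, so its speed depends on frame rate.
; The construction script randomizes the cylinder's starting yaw.
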(event Custom|Start%20Rotation
  (Rendering|SetVisibility (Variables|Default|GetSpotLight) true false)
  (Utilities|FlowControl|Gate true) ; enters at Open
)

(event Custom|Stop%20Rotation
  (Rendering|SetVisibility (Variables|Default|GetSpotLight) false false)
  (Utilities|FlowControl|Gate true) ; enters at Close
)

(event EventTick
  (params (DeltaSeconds :type Float%20%28single-precision%29))
  (Utilities|FlowControl|Gate true
    (:Exit
      (Transformation|AddRelativeRotation (Variables|Default|GetCylinder) "0.000000,4.000000,0.000000" false false))))

(fn ConstructionScript
  (Transformation|SetRelativeRotation (Variables|Default|GetCylinder) (Math|Rotator|MakeRotator 0.0 0.0 (Math|Random|RandomFloatinRange -179.0 1.8e+02)) false false))