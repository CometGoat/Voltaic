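; Networked bouncing projectile that damages players other than its firer, with particle, light and sound effects tinted by ParticleColour where applicable.
; On BeginPlay it applies the colour and adds itself to the ETC_GameState projectile list.
; The server counts down bounces, then multicasts component removal, sound fade and delayed destruction.
; Overlaps clear the victim's indicator widget, while the server applies damage and multicasts coloured sparks without destroying the projectile.
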(event OnComponentBeginOverlap(ProjectileCollision)
  (params (OverlappedComponent :type Primitive%20Component%20Object%20Reference) (OtherActor :type Actor%20Object%20Reference) (OtherComp :type Primitive%20Component%20Object%20Reference) (OtherBodyIndex :type Integer) (bFromSweep :type Boolean) (SweepResult :type Hit%20Result%20Structure%20%28by%20ref%29))
  (bind _asetcplayer_character (Utilities|Casting|CastToETCPlayerCharacter (Variables|/Script/Engine.Actor|GetInstigator OtherActor))
    (:then
      ;[1 1 1] Detecting Hits
      (bind _asetcplayer_character_2 (Utilities|Casting|CastToETCPlayerCharacter (Components|GetOwner))
        (:then
          (if (not (== _asetcplayer_character _asetcplayer_character_2))
            (Utilities|IsValid (Variables|/Game/Player/Pawns/ETCPlayerCharacter.ETCPlayerCharacter_C|GetPlayerIndicatorWidget _asetcplayer_character)
              (:Is%20Valid
                (Default|Remove (Variables|/Game/Player/Pawns/ETCPlayerCharacter.ETCPlayerCharacter_C|GetPlayerIndicatorWidget _asetcplayer_character)))
              (:Is%20Not%20Valid
                _))
            (Networking|SwitchHasAuthority
              (:Authority
                (Utilities|IsValid OtherActor
                  (:Is%20Valid
                    (Game|Damage|ApplyDamage OtherActor 1.0 (Game|GetInstigatorController) 0)
                    (CallFunction|ServerSpawnSparks)))))))
        (:CastFailed
          (Development|PrintString "Cast to firing character failed"))))
    (:CastFailed
      (Development|PrintString "Cast to instigator failed"))))

(event OnProjectileBounce(ProjectileMovement)
  (params (ImpactResult :type Hit%20Result%20Structure%20%28by%20ref%29) (ImpactVelocity :type Vector%20%28by%20ref%29 :default "0, 0, 0"))
  ;[1 1 1] Counting Bounces
  (Networking|SwitchHasAuthority
    (:Authority
      (if (Utilities|IsValid (.HitActor (Collision|BreakHitResult ImpactResult)))
        (Variables|Default|SetNumberOfBounces (- (Variables|Default|GetNumberOfBounces) 1))
        (Effects|SpawnEmitteratLocation "/Game/Effects/Particles/P_Ricochet.P_Ricochet" (Transformation|GetActorLocation) (Transformation|GetActorRotation))
        (if (<= (Variables|Default|GetNumberOfBounces) 0)
          (CallFunction|MulticastDestroyActor))))))

(event Custom|Multicast_DestroyActor
  ;[1 1 1] Counting Bounces
  (Components|DestroyComponent (Variables|Default|GetProjectileMesh))
  (Audio|Components|Audio|FadeOut (Variables|Default|GetProjectileSound) 1.0 0.0 :!class /Script/Engine.AudioComponent)
  (Utilities|FlowControl|Delay 2.0)
  (Actor|DestroyActor))

(event Custom|Server_SpawnSparks
  (CallFunction|MulticastSpawnSparks))

(event Custom|Multicast_SpawnSparks
  (bind _returnvalue (Transformation|GetActorRotation))
  (bind (_roll _pitch _yaw) (Math|Rotator|BreakRotator _returnvalue))
  (bind _returnvalue_2 (Effects|SpawnEmitteratLocation "/Game/Effects/Particles/P_DeathParticle_2.P_DeathParticle_2" (Transformation|GetActorLocation) (Math|Rotator|MakeRotator _roll _pitch _yaw)))
  (Effects|Components|ParticleSystem|SetColorParameter _returnvalue_2 "SparkColour" (Variables|Default|GetParticleColour)))

(event EventBeginPlay
  (bind _particlecolour (Variables|Default|GetParticleColour))
  ;[1 1 1] Set Projectile Ribbon Color
  (Audio|Components|Audio|Play (Variables|Default|GetProjectileSound) 0.0)
  (Effects|Components|ParticleSystem|SetColorParameter (Variables|Default|GetParticleSystem) "TeamColor" _particlecolour)
  (Rendering|Components|Light|SetLightColor (Variables|Default|GetPointLight) _particlecolour true)
  ;[1 1 1] Add Self to ProjectileList
  (bind _asetc_game_state (Utilities|Casting|CastToETC_GameState (Game|GetGameState)))
  (Variables|/Game/Gameplay/GameStates/ETC_GameState.ETC_GameState_C|SetProjectileToAdd _asetc_game_state self)
  (Default|AddtoProjectileList _asetc_game_state))

(event EventDestroyed
  (Audio|Components|Audio|FadeOut (Variables|Default|GetProjectileSound) 0.1 0.0 :!class /Script/Engine.AudioComponent))

(fn ConstructionScript
  ;[1 1 1] Always spawns on the server because of how we are spawning projectiles
)