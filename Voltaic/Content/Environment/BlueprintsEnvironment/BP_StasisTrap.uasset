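; BP_StasisTrap is a team-coloured projectile that deploys a BP_StasisSphere where it hits an actor.
; A hit triggers multicast effects that spawn the sphere, remove the ribbon particles, turn the mesh emissive red and swap the sound.
; A looping timer polls the sphere and multicasts a sound fade and self-destroy once it is gone.
; The overlap handler only performs casts, as its attach-to-player logic is disconnected, like the hit authority check.
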(event OnComponentBeginOverlap(ProjectileCollision)
  (params (OverlappedComponent :type Primitive%20Component%20Object%20Reference) (OtherActor :type Actor%20Object%20Reference) (OtherComp :type Primitive%20Component%20Object%20Reference) (OtherBodyIndex :type Integer) (bFromSweep :type Boolean) (SweepResult :type Hit%20Result%20Structure%20%28by%20ref%29))
  (bind _asetcplayer_character (Utilities|Casting|CastToETCPlayerCharacter (Variables|/Script/Engine.Actor|GetInstigator OtherActor))
    (:then
      (bind _asetcplayer_character_2 (Utilities|Casting|CastToETCPlayerCharacter (Components|GetOwner))
        (:CastFailed
          (Development|PrintString "Cast to firing character failed"))))
    (:CastFailed
      (Development|PrintString "Cast to instigator failed"))))

(event OnComponentHit(ProjectileCollision)
  (params (HitComponent :type Primitive%20Component%20Object%20Reference) (OtherActor :type Actor%20Object%20Reference) (OtherComp :type Primitive%20Component%20Object%20Reference) (NormalImpulse :type Vector :default "0, 0, 0") (Hit :type Hit%20Result%20Structure%20%28by%20ref%29))
  ;[1 1 1] Counting Bounces
  (if (Utilities|IsValid (.HitActor (Collision|BreakHitResult Hit)))
    (CallFunction|MulticastEffects)
    (Utilities|Time|SetTimerbyEvent (delegate Custom|Checking%20If%20Emitter%20Has%20Finished) 0.1 true)))

(event Custom|Multicast_DestroyActor
  ;[1 1 1] Counting Bounces
  (Audio|Components|Audio|FadeOut (Variables|Default|GetProjectileSound) 1.0 0.0 :!class /Script/Engine.AudioComponent)
  (Utilities|FlowControl|Delay 1.2)
  (Actor|DestroyActor))

(event Custom|Checking%20If%20Emitter%20Has%20Finished
  (Utilities|IsValid (stale Custom|Multicast_Effects _returnvalue)
    (:Is%20Not%20Valid
      (CallFunction|MulticastDestroyActor))))

(event Custom|Multicast_Effects
  (bind _projectilesound (Variables|Default|GetProjectileSound))
  ;[1 1 1] Counting Bounces
  (bind _returnvalue (Game|SpawnActorfromClass "/Game/Environment/BlueprintsEnvironment/BP_StasisSphere.BP_StasisSphere_C" (Transformation|GetActorTransform) "Undefined" self (Variables|Default|GetParticleColour) 0))
  (Components|DestroyComponent (Variables|Default|GetParticleSystem))
  (Rendering|Material|SetMaterial (Variables|Default|GetProjectileMesh) 0 "/Game/Environment/Materials/WallMaterials/M_EmissiveRed.M_EmissiveRed")
  (Audio|Components|Audio|FadeOut (Variables|Default|GetProjectileSound) 0.5 0.0 :!class /Script/Engine.AudioComponent)
  (Utilities|FlowControl|Delay 0.5)
  (Audio|Components|Audio|SetSound _projectilesound 0)
  (Audio|Components|Audio|Play _projectilesound 0.0))

(event EventBeginPlay
  ;[1 1 1] Set Projectile Ribbon Color
  (Audio|Components|Audio|Play (Variables|Default|GetProjectileSound) 0.0)
  (Effects|Components|ParticleSystem|SetColorParameter (Variables|Default|GetParticleSystem) "TeamColor" (Variables|Default|GetRibbonColour)))

(fn ConstructionScript
  ;[1 1 1] Always spawns on the server because of how we are spawning projectiles
)