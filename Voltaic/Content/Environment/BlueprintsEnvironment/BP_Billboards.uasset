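; BP_Billboards is an environment billboard with a configurable mesh and an animated, hit-reactive screen material.
; The construction script creates a dynamic instance of M_ScreenWarning_Inst, which the events drive through scalar parameters.
; ChangeBillboardImage starts a looping timer that steps AnimationPhase down each second, then stops and resets it.
; Any hit switches on the Static effect until a retriggerable one-second delay expires; a projectile-type filter is left disconnected.
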(event OnComponentHit(Billboard)
  (params (HitComponent :type Primitive%20Component%20Object%20Reference) (OtherActor :type Actor%20Object%20Reference) (OtherComp :type Primitive%20Component%20Object%20Reference) (NormalImpulse :type Vector :default "0, 0, 0") (Hit :type Hit%20Result%20Structure%20%28by%20ref%29))
  (Rendering|Material|SetScalarParameterValue (Variables|Default|GetBillboardMaterial) "Static" 1.0 :!class /Script/Engine.MaterialInstanceDynamic)
  (Utilities|FlowControl|RetriggerableDelay 1.0)
  (Rendering|Material|SetScalarParameterValue (Variables|Default|GetBillboardMaterial) "Static" 0.0 :!class /Script/Engine.MaterialInstanceDynamic))

(event Custom|Change%20Billboard%20Image
  (Rendering|Material|SetScalarParameterValue (Variables|Default|GetBillboardMaterial) "SignAnimate" 1.0 :!class /Script/Engine.MaterialInstanceDynamic)
  (bind _returnvalue (Utilities|Time|SetTimerbyEvent (delegate Custom|BeginCountdown) 1.0 true))
  (Variables|Default|SetCountdownHandler _returnvalue))

(event Custom|BeginCountdown
  (if (<= (Variables|Default|GetAnimationPhaseValue) 0.1)
    (Utilities|Time|ClearandInvalidateTimerbyHandle (Variables|Default|GetCountdownHandler))
    (Rendering|Material|SetScalarParameterValue (Variables|Default|GetBillboardMaterial) "SignAnimate" 0.0 :!class /Script/Engine.MaterialInstanceDynamic)
    (bind _output_get (Variables|Default|SetAnimationPhaseValue 0.9))
    (Rendering|Material|SetScalarParameterValue (Variables|Default|GetBillboardMaterial) "AnimationPhase" _output_get :!class /Script/Engine.MaterialInstanceDynamic)
    (else
      (Variables|Default|SetAnimationPhaseValue (- (Variables|Default|GetAnimationPhaseValue) 0.1))
      (Rendering|Material|SetScalarParameterValue (Variables|Default|GetBillboardMaterial) "AnimationPhase" (Variables|Default|GetAnimationPhaseValue) :!class /Script/Engine.MaterialInstanceDynamic))))

(fn ConstructionScript
  (Utilities|FlowControl|Sequence
    (:then_0
      (bind _returnvalue (Rendering|Material|CreateDynamicMaterialInstance (Variables|Default|GetBillboard) 1 "/Game/Environment/Materials/M_ScreenWarning_Inst.M_ScreenWarning_Inst" :!class /Script/Engine.PrimitiveComponent))
      (Variables|Default|SetBillboardMaterial _returnvalue))
    (:then_1
      (Components|StaticMesh|SetStaticMesh (Variables|Default|GetBillboard) (Variables|Default|GetBillboardMesh)))))