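; Bouncing, team-coloured projectile for the Split game variant that registers itself with the game state on spawn.
; Each bounce spends a count and spawns a ricochet effect; at zero it strips its components, fades audio, then destroys itself.
; Overlaps damage other characters and trigger double/triple kill announcements from a per-projectile count.
; Overlaps with the firer's own character take a reflect path intended to turn the projectile around when dodging.
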(event OnComponentBeginOverlap(ProjectileCollision)
  (params (OverlappedComponent :type Primitive%20Component%20Object%20Reference) (OtherActor :type Actor%20Object%20Reference) (OtherComp :type Primitive%20Component%20Object%20Reference) (OtherBodyIndex :type Integer) (bFromSweep :type Boolean) (SweepResult :type Hit%20Result%20Structure%20%28by%20ref%29))
  (bind _returnvalue (Components|GetOwner))
  (bind _returnvalue_2 (Game|GetGameMode))
  (bind _asetc_game_mode_split (Utilities|Casting|CastToETC_GameMode_Split _returnvalue_2))
  (bind _asetcplayer_character_split (Utilities|Casting|CastToETCPlayerCharacter_Split (Variables|/Script/Engine.Actor|GetInstigator OtherActor))
    (:then
      (Utilities|IsValid _returnvalue
        (:Is%20Valid
          (bind _asetcplayer_character_split_2 (Utilities|Casting|CastToETCPlayerCharacter_Split _returnvalue))
          ;[1 1 1] Detecting Hits
          (if (== _asetcplayer_character_split _asetcplayer_character_split_2)
            (CallFunction|ReflectOwnTeam)
            (else
              (Utilities|IsValid (Variables|/Game/Player/Pawns/ETCPlayerCharacter_Split.ETCPlayerCharacter_Split_C|GetPlayerIndicatorWidget _asetcplayer_character_split) :!label _label
                (:Is%20Valid
                  (Default|Remove (Variables|/Game/Player/Pawns/ETCPlayerCharacter_Split.ETCPlayerCharacter_Split_C|GetPlayerIndicatorWidget _asetcplayer_character_split)))
                (:Is%20Not%20Valid
                  _))
              (Utilities|IsValid OtherActor
                (:Is%20Valid
                  (Game|Damage|ApplyDamage OtherActor 1.0 (Game|GetInstigatorController) self)
                  (bind _returnvalue_3 (Effects|SpawnEmitteratLocation "/Game/Effects/Particles/P_DeathParticle_2.P_DeathParticle_2" (Transformation|GetActorLocation)))
                  (Effects|Components|ParticleSystem|SetColorParameter _returnvalue_3 "SparkColour" (Variables|Default|GetParticleColour))
                  (bind _output_get (Variables|Default|SetKillCount (+ (Variables|Default|GetKillCount) 1)))
                  (if (== _output_get 2)
                    (Default|AnnouncerDoubleKill _asetc_game_mode_split)
                    (elif (== _output_get 3)
                      (Default|AnnouncerTripleKill _asetc_game_mode_split))))))))
        (:Is%20Not%20Valid
          (goto _label))))
    (:CastFailed
      (Development|PrintString "Cast to instigator failed"))))

(event OnProjectileBounce(ProjectileMovement)
  (params (ImpactResult :type Hit%20Result%20Structure%20%28by%20ref%29) (ImpactVelocity :type Vector%20%28by%20ref%29 :default "0, 0, 0"))
  ;[1 1 1] Counting Bounces
  (if (Utilities|IsValid (.HitActor (Collision|BreakHitResult ImpactResult)))
    (Variables|Default|SetNumberOfBounces (- (Variables|Default|GetNumberOfBounces) 1))
    (Effects|SpawnEmitteratLocation "/Game/Effects/Particles/P_Ricochet.P_Ricochet" (Transformation|GetActorLocation) (Transformation|GetActorRotation))
    (if (<= (Variables|Default|GetNumberOfBounces) 0)
      (CallFunction|DestroyActor))))

(event Custom|DestroyActor
  ;[1 1 1] Counting Bounces
  (Components|DestroyComponent (Variables|Default|GetProjectileMesh))
  (Audio|Components|Audio|FadeOut (Variables|Default|GetProjectileSound) 1.0 0.0 :!class /Script/Engine.AudioComponent)
  (Utilities|FlowControl|Delay 2.0)
  (Actor|DestroyActor))

(event Custom|Reflect_OwnTeam
  (params (Character :type ETC%20Player%20Character%20Split%20Object%20Reference))
  (if (and (Variables|/Game/Player/Pawns/ETCPlayerCharacter_Split.ETCPlayerCharacter_Split_C|GetDodging? Character) (not (Variables|Default|GetReflectedOwnTeam)))
    (Variables|Default|SetReflectedOwnTeam true)
    (Variables|/Script/Engine.MovementComponent|SetVelocity (Variables|Default|GetProjectileMovement) (Math|Vector|RotateVector (Transformation|GetVelocity) "0.000000,180.000000,0.000000"))
    (Utilities|FlowControl|Delay 0.2)
    (Variables|Default|SetReflectedOwnTeam false)))

(event EventBeginPlay
  (bind _particlecolour (Variables|Default|GetParticleColour))
  ;[1 1 1] Set Projectile Ribbon Color
  (Variables|Default|SetOwningPlayerController (Pawn|GetController (Variables|/Script/Engine.Actor|GetInstigator (Components|GetOwner))))
  (Audio|Components|Audio|Play (Variables|Default|GetProjectileSound) 0.0)
  (Effects|Components|ParticleSystem|SetColorParameter (Variables|Default|GetParticleSystem) "TeamColor" _particlecolour)
  (Rendering|Components|Light|SetLightColor (Variables|Default|GetPointLight) _particlecolour true)
  ;[1 1 1] Add Self to ProjectileList
  (bind _asetc_game_state_split (Utilities|Casting|CastToETC_GameState_Split (Game|GetGameState)))
  (Variables|/Game/Gameplay/GameStates/ETC_GameState_Split.ETC_GameState_Split_C|SetProjectileToAdd _asetc_game_state_split self)
  (Default|AddtoProjectileList _asetc_game_state_split))

(event EventDestroyed
  (Audio|Components|Audio|FadeOut (Variables|Default|GetProjectileSound) 0.1 0.0 :!class /Script/Engine.AudioComponent))

(fn ConstructionScript
  ;[1 1 1] Always spawns on the server because of how we are spawning projectiles
)

(fn ReflectOffPlayer
  (params (Character :type ETC%20Player%20Character%20Split%20Object%20Reference)))