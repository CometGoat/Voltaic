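; BP_ClosingDoors is an environment actor with two sliding doors that animate shut or open through CloseDoors and OpenDoors events.
; On BeginPlay it caches each door's world location as open and the StaticMesh location as the shared closed point.
; Both events set a Closing flag and restart one timeline, whose separate Close and Open tracks drive the position lerps.
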(event Custom|CloseDoors
  (Variables|Default|SetClosing true)
  (bind (_direction _close _open) (Timeline|ClosingDoors PlayFromStart)
    (:Update
      (if (Variables|Default|GetClosing)
        (Transformation|SetWorldLocation (Variables|Default|GetLeftDoor) (Math|Vector|Lerp(Vector) (Variables|Default|GetLeftDoorOpen) (Variables|Default|GetDoorsClosed) _close) false false)
        (Transformation|SetWorldLocation (Variables|Default|GetRightDoor) (Math|Vector|Lerp(Vector) (Variables|Default|GetRightDoorOpen) (Variables|Default|GetDoorsClosed) _close) false false)
        (else
          (Transformation|SetWorldLocation (Variables|Default|GetLeftDoor) (Math|Vector|Lerp(Vector) (Variables|Default|GetDoorsClosed) (Variables|Default|GetLeftDoorOpen) _open) false false)
          (Transformation|SetWorldLocation (Variables|Default|GetRightDoor) (Math|Vector|Lerp(Vector) (Variables|Default|GetDoorsClosed) (Variables|Default|GetRightDoorOpen) _open) false false))))))

(event Custom|OpenDoors
  (Variables|Default|SetClosing false)
  (bind (_direction _close _open) (Timeline|ClosingDoors PlayFromStart)
    (:Update
      (if (Variables|Default|GetClosing)
        (Transformation|SetWorldLocation (Variables|Default|GetLeftDoor) (Math|Vector|Lerp(Vector) (Variables|Default|GetLeftDoorOpen) (Variables|Default|GetDoorsClosed) _close) false false)
        (Transformation|SetWorldLocation (Variables|Default|GetRightDoor) (Math|Vector|Lerp(Vector) (Variables|Default|GetRightDoorOpen) (Variables|Default|GetDoorsClosed) _close) false false)
        (else
          (Transformation|SetWorldLocation (Variables|Default|GetLeftDoor) (Math|Vector|Lerp(Vector) (Variables|Default|GetDoorsClosed) (Variables|Default|GetLeftDoorOpen) _open) false false)
          (Transformation|SetWorldLocation (Variables|Default|GetRightDoor) (Math|Vector|Lerp(Vector) (Variables|Default|GetDoorsClosed) (Variables|Default|GetRightDoorOpen) _open) false false))))))

(event EventBeginPlay
  (CallFunction|SetDoorLocations))

(fn ConstructionScript)

(fn SetDoorLocations
  (Variables|Default|SetLeftDoorOpen (Transformation|GetWorldLocation (Variables|Default|GetLeftDoor)))
  (Variables|Default|SetRightDoorOpen (Transformation|GetWorldLocation (Variables|Default|GetRightDoor)))
  (Variables|Default|SetDoorsClosed (Transformation|GetWorldLocation (Variables|Default|GetStaticMesh))))