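; Map 2 event manager that runs a randomized countdown to an acid hazard, with doors closing ahead of it.
; BeginPlay gathers acid and door actors, picks a random time, then re-checks the game state until it allows the countdown.
; A Tick-fed Gate counts down, and a DoOnce closes all doors in the final seconds.
; At zero it activates every acid actor with itself as owning event.
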(event Custom|BeginCountdown
  ;[1 1 1] Timer counting down to hazard event
  (Utilities|FlowControl|Gate true) ; enters at Open
)

(event EventBeginPlay
  ;[1 1 1] Getting all doors and acid actors on the map
  (bind _outactors (Actor|GetAllActorsOfClass "/Game/Environment/BlueprintsEnvironment/Map2Event/AcidActor.AcidActor_C"))
  (Variables|Default|SetAcidActor _outactors)
  (bind _outactors_2 (Actor|GetAllActorsOfClass "/Game/Environment/BlueprintsEnvironment/Map2Event/ClosingDoors_BP.ClosingDoors_BP_C"))
  (Variables|Default|SetDoorBPs _outactors_2)
  ;[1 1 1] Sets intial Timer
  (CallFunction|SetTimer)
  ;[1 0 0] This could be done with an event dispatcher, will redo.
  (bind _asetc_game_state (Utilities|Casting|CastToETC_GameState (Game|GetGameState) :!label _label)
    (:then
      (if (Utilities|Enum|Equal(Enum) (Variables|/Game/Gameplay/GameStates/ETC_GameState.ETC_GameState_C|GetGameplayState _asetc_game_state) "NewEnumerator2")
        (CallFunction|BeginCountdown)
        (Development|PrintString "BeginCountdownWorked")
        (else
          (goto _label))))
    (:CastFailed
      (Development|PrintString "Event Failed to cast"))))

(event EventTick
  (params (DeltaSeconds :type Float%20%28single-precision%29))
  ;[1 1 1] Timer counting down to hazard event
  (if (not (Variables|Default|GetEventActive))
    (Utilities|FlowControl|Gate true
      (:Exit
        (bind _output_get (Variables|Timer|SetTimeRemaining (Math|Float|Max(Float) (- (Variables|Timer|GetTimeRemaining) DeltaSeconds) 0.0)))
        (if (<= _output_get 0.0)
          ;[1 1 1] Activating events associated with hazards
          (Variables|Default|SetEventActive true)
          (for _array_element (Variables|Default|GetAcidActor)
            (Variables|/Game/Environment/BlueprintsEnvironment/Map2Event/AcidActor.AcidActor_C|SetOwningEvent (.AsAcid%20Actor (Utilities|Casting|CastToAcidActor _array_element)) self)
            (Default|ActivateHazard (.AsAcid%20Actor (Utilities|Casting|CastToAcidActor _array_element)))
            (Development|PrintString "Activated Hazard"))
          (goto _label Reset)
          (elif (<= (Variables|Timer|GetTimeRemaining) 7.0)
            (Utilities|FlowControl|DoOnce false :!label _label
              (:Completed
                (for _array_element_2 (Variables|Default|GetDoorBPs)
                  (Default|CloseDoors (.AsClosing%20Doors%20BP (Utilities|Casting|CastToClosingDoors_BP _array_element_2))))))))))))

(fn ConstructionScript)

(fn SetTimer
  (Variables|Timer|SetTimeRemaining (Math|Conversions|ToFloat(Integer) (Math|Float|Truncate (Math|Random|RandomFloatinRange (Variables|Timer|GetMinTimeBeforeEvent) (Variables|Timer|GetMaxTimeBeforeEvent)))))
  (Variables|Default|SetEventActive false))