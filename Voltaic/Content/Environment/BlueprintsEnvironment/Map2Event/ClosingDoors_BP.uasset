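; Map 2 event actor that slides a pair of doors shut when its CloseDoors event is called.
; BeginPlay caches each door's starting world location as open and derives closed positions offset in opposite directions along world X, so actor rotation is ignored.
; CloseDoors plays the ClosingDoors timeline from the start, lerping both doors between those positions without sweep.
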(event Custom|CloseDoors
  (bind _movement (Timeline|ClosingDoors PlayFromStart)
    (:Update
      (Transformation|SetWorldLocation (Variables|Default|GetLeftDoor) (Math|Vector|Lerp(Vector) (Variables|Default|GetLeftDoorOpen) (Variables|Default|GetLeftDoorClosed) _movement) false false)
      (Transformation|SetWorldLocation (Variables|Default|GetRightDoor) (Math|Vector|Lerp(Vector) (Variables|Default|GetRightDoorOpen) (Variables|Default|GetRightDoorClosed) _movement) false false))))

(event EventBeginPlay
  (CallFunction|SetDoorLocations))

(fn ConstructionScript)

(fn SetDoorLocations
  (bind _rightdoor (Variables|Default|GetRightDoor))
  (bind _leftdoor (Variables|Default|GetLeftDoor))
  (bind _returnvalue (Transformation|GetWorldLocation _rightdoor))
  (bind _returnvalue_2 (Transformation|GetWorldLocation _leftdoor))
  (Variables|Default|SetLeftDoorOpen _returnvalue_2)
  (Variables|Default|SetLeftDoorClosed (+ _returnvalue_2 "150.000000, 0, 0"))
  (Variables|Default|SetRightDoorOpen _returnvalue)
  (Variables|Default|SetRightDoorClosed (- _returnvalue "150.000000, 0, 0")))